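; Zombie spawner actor that spawns test zombies at its own transform while a player is nearby.
; Begin and end overlap events check the overlapping actor against player pawns in the game state's PlayerArray to toggle AllowSpawning.
; On the server, Tick runs a one-second Delay while spawning is allowed, then spawns a TestZombieBP until the spawned count reaches MaxSpawnableZombies.
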(event `self.ReceiveActorBeginOverlap`
  (params (OtherActor :type "Actor Object Reference"))
  (for _array_element (`GameStateBase.PlayerArray` (`GameplayStatics.GetGameState`))
    (if (== OtherActor (`PlayerState.PawnPrivate` _array_element))
      (set `self.allowSpawning` true)
      (break))))

(event `self.ReceiveActorEndOverlap`
  (params (OtherActor :type "Actor Object Reference"))
  (for _array_element (`GameStateBase.PlayerArray` (`GameplayStatics.GetGameState`))
    (if (== OtherActor (`PlayerState.PawnPrivate` _array_element))
      (set `self.allowSpawning` false)
      (break))))

(event `self.ReceiveTick`
  (params (DeltaSeconds :type "Float (single-precision)"))
  (`/Engine/EditorBlueprintResources/ActorMacros.Switch Has Authority`
    (:`Authority`
      (if (`self.allowSpawning`)
        (`KismetSystemLibrary.Delay` 1.0)
        (if (< (`self.zombiesSpawned`) (`self.maxSpawnableZombies`))
          (`|SpawnActorFromClass` "/Game/Zombies/Blueprints/TestZombieBP.TestZombieBP_C" (`self.GetTransform`) "AdjustIfPossibleButAlwaysSpawn" "OverrideRootScale" null null)
          (`/Engine/EditorBlueprintResources/StandardMacros.IncrementInt` (`self.zombiesSpawned`)))))))

(fn `UserConstructionScript`)